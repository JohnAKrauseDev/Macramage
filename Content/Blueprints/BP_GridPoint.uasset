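; Grid point actor that stores its grid index and can briefly highlight its cube.
; HighlightPoint swaps the cube to the highlighted material and sets a short timer by function name to call StopHighlightPoint, which restores the unhighlighted material.
; Repeated calls reset that timer, so the highlight holds while calls keep arriving.
; GetIndex returns the stored GridIndex with an always-true success flag, and the event graph is unused.
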(event EventBeginPlay)

(event Collision|EventActorBeginOverlap
  (params (OtherActor :type Actor%20Object%20Reference)))

(event EventTick
  (params (DeltaSeconds :type Float%20%28single-precision%29)))

(fn ConstructionScript)

(fn HighlightPoint
  (Rendering|Material|SetMaterial (Variables|Default|GetCube) 0 (Variables|Default|GetHighlightedMaterial))
  (Utilities|Time|SetTimerbyFunctionName 0 "StopHighlightPoint" 0.05))

(fn StopHighlightPoint
  (Rendering|Material|SetMaterial (Variables|Default|GetCube) 0 (Variables|Default|GetUnhiglightedMaterial)))

(fn GetIndex
  (return true (Variables|Default|GetGridIndex)))