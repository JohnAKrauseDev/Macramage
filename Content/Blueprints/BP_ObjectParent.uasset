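; BP_ObjectParent is the base actor for damageable objects on the Macramage grid, with configurable mesh, scale, sprite and a bar widget linked back to it.
; Move stores the new grid point and lerps the actor there on a Timeline.
; RecieveAttack reduces Health; death runs the empty ExtraEffectOnDeath hook, frees the grid point, leaves the controller's ObjectArray and destroys the actor.
; Status effects only print a placeholder message here.
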(event Custom|Move
  (params (NewLocation :type Vector) (newGridPoint :type Integer))
  (Variables|Default|SetCurrentGridPoint newGridPoint)
  (Variables|Default|SetOldLocation (Transformation|GetActorLocation))
  (bind _newtrack_0 (Timeline|Timeline PlayFromStart)
    (:Update
      (Transformation|SetActorLocation (Math|Vector|Lerp(Vector) (Variables|Default|GetOldLocation) NewLocation _newtrack_0) false false))))

(event EventBeginPlay
  (bind _asobject_uibars (Utilities|Casting|CastToObjectUibars (UserInterface|GetWidget (Variables|Default|GetWidget))))
  (Variables|/Game/Blueprints/ObjectUibars.ObjectUibars_C|SetParentObjectRef _asobject_uibars self))

(fn ConstructionScript
  (bind _staticmesh (Variables|Default|GetStaticMesh))
  (Components|StaticMesh|SetStaticMesh _staticmesh (Variables|Default|GetMesh))
  (Transformation|SetRelativeScale3D _staticmesh (Math|Conversions|ToVector(Float) (Variables|Default|GetMeshScale)))
  (Rendering|Components|Sprite|SetSprite (Variables|Default|GetPaperSprite) (Variables|Default|GetSprite)))

(fn RecieveAttack
  (params (Damage :type Integer) (StatusEffects :type Array%20of%20EnemyStatusEnum%20Enums :default "NewEnumerator0"))
  (Variables|Default|SetHealth (- (Variables|Default|GetHealth) Damage))
  (bind _isdead (CallFunction|CheckifDead))
  (if _isdead
    (CallFunction|Die)
    (elif (Utilities|Array|IsNotEmpty StatusEffects)
      (Development|PrintString "BP_Object base, doesnt know what to sdo ewith status effect in recieve attacvk"))))

(fn CheckifDead
  (if (<= (Variables|Default|GetHealth) 0)
    (bind _asbp_macramage_controller (Utilities|Casting|CastToBP_Macramage_Controller (Game|GetPlayerController 0)))
    (Utilities|Array|RemoveItem (Variables|/Game/Blueprints/Player/BP_Macramage_Controller.BP_Macramage_Controller_C|GetObjectArray _asbp_macramage_controller) self)
    (return true)
    (else
      (return false))))

(fn ExtraEffectonDeath)

(fn Die
  ;[1 0 0] CHECK FOR EXTRA EFECT ON DEATH
  (CallFunction|ExtraEffectonDeath)
  ;[1 1 1] Set grid point not occupied
  (bind _asbp_macramage_controller (Utilities|Casting|CastToBP_Macramage_Controller (Game|GetPlayerController 0)))
  (bind _keys (Utilities|Map|Keys (Variables|/Game/Blueprints/BP_Grid.BP_Grid_C|GetGridPoints (Variables|/Game/Blueprints/Player/BP_Macramage_Controller.BP_Macramage_Controller_C|GetGridReference _asbp_macramage_controller))))
  (Utilities|Map|Add (Variables|/Game/Blueprints/BP_Grid.BP_Grid_C|GetGridPoints (Variables|/Game/Blueprints/Player/BP_Macramage_Controller.BP_Macramage_Controller_C|GetGridReference _asbp_macramage_controller)) (Utilities|Array|Get(acopy) _keys (Variables|Default|GetCurrentGridPoint)) false)
  (Utilities|Array|RemoveItem (Variables|/Game/Blueprints/Player/BP_Macramage_Controller.BP_Macramage_Controller_C|GetObjectArray _asbp_macramage_controller) self)
  ;;[1 1 1] Die
  (Actor|DestroyActor))