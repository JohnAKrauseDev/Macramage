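; BP_Grid builds a row-by-column grid of points from GridStart and registers itself with the Macramage player controller on BeginPlay.
; RefreshGridIndecators destroys old points and indicators, then adds scene components as keys in the GridPoints map, each with a false value.
; It optionally spawns indexed BP_GridPoint indicator actors above them.
; The construction script can rebuild it in-editor, while BeginPlay rebuilds and sets in-game indicator visibility.
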(event EventBeginPlay
  (CallFunction|RefreshGrid+Indecators true)
  (bind _asbp_macramage_controller (Utilities|Casting|CastToBP_Macramage_Controller (Game|GetPlayerController 0)))
  (Variables|/Game/Blueprints/Player/BP_Macramage_Controller.BP_Macramage_Controller_C|SetGridReference _asbp_macramage_controller self))

(event Collision|EventActorBeginOverlap
  (params (OtherActor :type Actor%20Object%20Reference)))

(event EventTick
  (params (DeltaSeconds :type Float%20%28single-precision%29)))

(fn ConstructionScript
  (if (Variables|Default|GetUpdateInOutline)
    (CallFunction|RefreshGrid+Indecators false)))

(fn RefreshGrid+Indecators
  (params (IsBeginPlay :type Boolean))
  ;[1 1 1] Clear old
  (bind _keys (Utilities|Map|Keys (Variables|Default|GetGridPoints)))
  (for _array_element _keys
    (Components|DestroyComponent _array_element))
  (for _array_element_2 (Variables|Default|GetGridPointIndecatiors)
    (Actor|DestroyActor _array_element_2))
  (bind _keys_2 (Utilities|Map|Keys (Variables|Default|GetGridPoints)))
  (Utilities|Array|Clear _keys_2)
  (Utilities|Array|Clear (Variables|Default|GetGridPointIndecatiors))
  (for _index (range 0 (- (Variables|Default|GetRows) 1))
    (for _index_2 (range 0 (- (Variables|Default|GetCollumns) 1))
      (bind _returnvalue (AddComponent|AddSceneComponent false (Math|Transform|MakeTransform (+ (Variables|/Script/Engine.SceneComponent|GetRelativeLocation (Variables|Default|GetGridStart)) (Math|Vector|MakeVector (* (Variables|Default|GetRowDistance) _index) (* _index_2 (Variables|Default|GetCollumnDistance)) 0.0)) "0, 0, 0" "1.000000,1.000000,1.000000")))
      (Utilities|Map|Add (Variables|Default|GetGridPoints) _returnvalue false)))
  (if (Variables|Default|GetShowIndecators)
    (bind _keys_3 (Utilities|Map|Keys (Variables|Default|GetGridPoints)))
    (for (_array_element_3 _array_index) _keys_3
      (bind _returnvalue_2 (Game|SpawnActorfromClass "/Game/Blueprints/BP_GridPoint.BP_GridPoint_C" (Math|Transform|MakeTransform (+ (Transformation|GetWorldLocation _array_element_3) (Math|Vector|MakeVector 0.0 0.0 (Variables|Default|GetIndecatorZOffset))) "0, 0, 0" "1.000000,1.000000,1.000000") "Undefined" "MultiplyWithRoot" 0 _array_index 0))
      (Utilities|Array|Add (Variables|Default|GetGridPointIndecatiors) _returnvalue_2)
      (if IsBeginPlay
        (Rendering|SetVisibility (Variables|/Script/Engine.Actor|GetRootComponent _returnvalue_2) (Variables|Default|GetShowInGameIndecators) true)))))