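; BP_Enemyparent is a parent enemy Blueprint for an actor that moves between grid points.
; The Move event records the new grid point, then uses a Timeline to lerp the actor from its current location to the target without sweeping.
; The construction script picks a placeholder-style static mesh, cone or cube, from the EnemyType value.
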(event Custom|Move
  (params (NewLocation :type Vector) (newGridPoint :type Integer))
  (Variables|Default|SetCurrentGridPoint newGridPoint)
  (Variables|Default|SetOldLocation (Transformation|GetActorLocation))
  (bind _newtrack_0 (Timeline|Timeline PlayFromStart)
    (:Update
      (Transformation|SetActorLocation (Math|Vector|Lerp(Vector) (Variables|Default|GetOldLocation) NewLocation _newtrack_0) false false))))

(fn ConstructionScript
  (switch Utilities|FlowControl|Switch|SwitchonMonsterEnum (Variables|Default|GetEnemyType)
    (:NewEnumerator1
      (Components|StaticMesh|SetStaticMesh (Variables|Default|GetStaticMesh) "/Engine/BasicShapes/Cone.Cone"))
    (:NewEnumerator2
      (Components|StaticMesh|SetStaticMesh (Variables|Default|GetStaticMesh) "/Engine/BasicShapes/Cube.Cube"))))