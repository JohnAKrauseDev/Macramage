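; MacramageGameInstance is the game instance that seeds the player's starting scarf spells and owned items at Init.
; It fills ScarfSpells with three default entries drawn from ItemsReferenceList.
; It then flattens each spell's Thread, Pattern and Extra slots into ScarfItems, skipping any named "None".
; Two further reference items are added to InventoryItems as extra starting inventory.
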(event EventInit
  (CallFunction|InitializScarfSpells)
  (CallFunction|InitializeOwnedItems))

(fn InitializScarfSpells
  (bind _itemsreferencelist (Variables|Default|GetItemsReferenceList))
  (bind _output (Utilities|Array|Get(acopy) _itemsreferencelist))
  (Utilities|Array|Add (Variables|Default|GetScarfSpells) (Utilities|Struct|MakeScarfSpellSlot _output "(ItemType_11_EE818EA24280422D72C2498698E08AE8=NewEnumerator0,Name_24_48D5A0354C41A9F8481BF9A1BA4E849C=\"\",ThreadInfo_20_AC64FCC341FDFECB20D32E9C93B024BC=(BaseBehavior_8_9CCA090A4406AA5AC5D519A460EEBEA6=NewEnumerator0,Damage_3_7136B4684F285CE98C584D9C7B6F1211=0,BaseEffect_14_BFB0B2B54DB8062F2023D3A3A52F01EF=NewEnumerator0,ExtraEffect_17_30B3C5A84F17E72B5B5AFDB8B99B8C71=NewEnumerator0),PatternInfo_9_113B66714E5732AF400BB6BBA624E069=(EffectedArea_7_1FE9FD4345555349B4C565B913FD64B4=),ExtraInfo_8_43FBA28143FF4C206A6BCB9FE977A8EB=(Effects_3_1CA141524E49CFD4619760BA32652630=),Image_17_22706E404D7BC7961BB83B8A4901D974=None,Color_18_353664D64C906E46DDF4939C464A62F8=(B=0,G=0,R=0,A=0))" "(ItemType_11_EE818EA24280422D72C2498698E08AE8=NewEnumerator0,Name_24_48D5A0354C41A9F8481BF9A1BA4E849C=\"\",ThreadInfo_20_AC64FCC341FDFECB20D32E9C93B024BC=(BaseBehavior_8_9CCA090A4406AA5AC5D519A460EEBEA6=NewEnumerator0,Damage_3_7136B4684F285CE98C584D9C7B6F1211=0,BaseEffect_14_BFB0B2B54DB8062F2023D3A3A52F01EF=NewEnumerator0,ExtraEffect_17_30B3C5A84F17E72B5B5AFDB8B99B8C71=NewEnumerator0),PatternInfo_9_113B66714E5732AF400BB6BBA624E069=(EffectedArea_7_1FE9FD4345555349B4C565B913FD64B4=),ExtraInfo_8_43FBA28143FF4C206A6BCB9FE977A8EB=(Effects_3_1CA141524E49CFD4619760BA32652630=),Image_17_22706E404D7BC7961BB83B8A4901D974=None,Color_18_353664D64C906E46DDF4939C464A62F8=(B=0,G=0,R=0,A=0))" false false))
  (Utilities|Array|Add (Variables|Default|GetScarfSpells) (Utilities|Struct|MakeScarfSpellSlot _output "(ItemType_11_EE818EA24280422D72C2498698E08AE8=NewEnumerator0,Name_24_48D5A0354C41A9F8481BF9A1BA4E849C=\"\",ThreadInfo_20_AC64FCC341FDFECB20D32E9C93B024BC=(BaseBehavior_8_9CCA090A4406AA5AC5D519A460EEBEA6=NewEnumerator0,Damage_3_7136B4684F285CE98C584D9C7B6F1211=0,BaseEffect_14_BFB0B2B54DB8062F2023D3A3A52F01EF=NewEnumerator0,ExtraEffect_17_30B3C5A84F17E72B5B5AFDB8B99B8C71=NewEnumerator0),PatternInfo_9_113B66714E5732AF400BB6BBA624E069=(EffectedArea_7_1FE9FD4345555349B4C565B913FD64B4=),ExtraInfo_8_43FBA28143FF4C206A6BCB9FE977A8EB=(Effects_3_1CA141524E49CFD4619760BA32652630=),Image_17_22706E404D7BC7961BB83B8A4901D974=None,Color_18_353664D64C906E46DDF4939C464A62F8=(B=0,G=0,R=0,A=0))" "(ItemType_11_EE818EA24280422D72C2498698E08AE8=NewEnumerator0,Name_24_48D5A0354C41A9F8481BF9A1BA4E849C=\"\",ThreadInfo_20_AC64FCC341FDFECB20D32E9C93B024BC=(BaseBehavior_8_9CCA090A4406AA5AC5D519A460EEBEA6=NewEnumerator0,Damage_3_7136B4684F285CE98C584D9C7B6F1211=0,BaseEffect_14_BFB0B2B54DB8062F2023D3A3A52F01EF=NewEnumerator0,ExtraEffect_17_30B3C5A84F17E72B5B5AFDB8B99B8C71=NewEnumerator0),PatternInfo_9_113B66714E5732AF400BB6BBA624E069=(EffectedArea_7_1FE9FD4345555349B4C565B913FD64B4=),ExtraInfo_8_43FBA28143FF4C206A6BCB9FE977A8EB=(Effects_3_1CA141524E49CFD4619760BA32652630=),Image_17_22706E404D7BC7961BB83B8A4901D974=None,Color_18_353664D64C906E46DDF4939C464A62F8=(B=0,G=0,R=0,A=0))" false false))
  (Utilities|Array|Add (Variables|Default|GetScarfSpells) (Utilities|Struct|MakeScarfSpellSlot (Utilities|Array|Get(acopy) (Variables|Default|GetItemsReferenceList) 1) "(ItemType_11_EE818EA24280422D72C2498698E08AE8=NewEnumerator0,Name_24_48D5A0354C41A9F8481BF9A1BA4E849C=\"\",ThreadInfo_20_AC64FCC341FDFECB20D32E9C93B024BC=(BaseBehavior_8_9CCA090A4406AA5AC5D519A460EEBEA6=NewEnumerator0,Damage_3_7136B4684F285CE98C584D9C7B6F1211=0,BaseEffect_14_BFB0B2B54DB8062F2023D3A3A52F01EF=NewEnumerator0,ExtraEffect_17_30B3C5A84F17E72B5B5AFDB8B99B8C71=NewEnumerator0),PatternInfo_9_113B66714E5732AF400BB6BBA624E069=(EffectedArea_7_1FE9FD4345555349B4C565B913FD64B4=),ExtraInfo_8_43FBA28143FF4C206A6BCB9FE977A8EB=(Effects_3_1CA141524E49CFD4619760BA32652630=),Image_17_22706E404D7BC7961BB83B8A4901D974=None,Color_18_353664D64C906E46DDF4939C464A62F8=(B=0,G=0,R=0,A=0))" "(ItemType_11_EE818EA24280422D72C2498698E08AE8=NewEnumerator0,Name_24_48D5A0354C41A9F8481BF9A1BA4E849C=\"\",ThreadInfo_20_AC64FCC341FDFECB20D32E9C93B024BC=(BaseBehavior_8_9CCA090A4406AA5AC5D519A460EEBEA6=NewEnumerator0,Damage_3_7136B4684F285CE98C584D9C7B6F1211=0,BaseEffect_14_BFB0B2B54DB8062F2023D3A3A52F01EF=NewEnumerator0,ExtraEffect_17_30B3C5A84F17E72B5B5AFDB8B99B8C71=NewEnumerator0),PatternInfo_9_113B66714E5732AF400BB6BBA624E069=(EffectedArea_7_1FE9FD4345555349B4C565B913FD64B4=),ExtraInfo_8_43FBA28143FF4C206A6BCB9FE977A8EB=(Effects_3_1CA141524E49CFD4619760BA32652630=),Image_17_22706E404D7BC7961BB83B8A4901D974=None,Color_18_353664D64C906E46DDF4939C464A62F8=(B=0,G=0,R=0,A=0))" false false)))

(fn InitializeOwnedItems
  (bind _inventoryitems (Variables|Default|GetInventoryItems))
  (bind _itemsreferencelist (Variables|Default|GetItemsReferenceList))
  ;[1 1 1] Get all the items in scarf
  (for _array_element (Variables|Default|GetScarfSpells)
    (Utilities|FlowControl|Sequence
      (:then_0
        (if (!= (.Name (Utilities|Struct|BreakItemStruct (.thread _array_element))) "None")
          (Utilities|Array|Add (Variables|Default|GetScarfItems) (.thread _array_element))))
      (:then_1
        (if (!= (.Name (Utilities|Struct|BreakItemStruct (.pattern _array_element))) "None")
          (Utilities|Array|Add (Variables|Default|GetScarfItems) (.pattern _array_element))))
      (:then_2
        (if (!= (.Name (Utilities|Struct|BreakItemStruct (.extra _array_element))) "None")
          (Utilities|Array|Add (Variables|Default|GetScarfItems) (.extra _array_element))))))
  ;[1 1 1] And any extras toi add to inv
  (Utilities|Array|Add _inventoryitems (Utilities|Array|Get(acopy) _itemsreferencelist 6))
  (Utilities|Array|Add _inventoryitems (Utilities|Array|Get(acopy) _itemsreferencelist 7)))