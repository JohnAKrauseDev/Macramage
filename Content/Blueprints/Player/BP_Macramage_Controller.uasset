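; Player controller for Macramage's grid-based turn combat, handling mouse aiming of Scarf spells and enemy wave logic.
; During the Aim phase, Tick traces under the cursor and highlights the current spell's tile shape within casting range, with optional edge wrapping.
; MovePhase advances enemies on the grid and SpawnPhase fills the back row from a data table, but their chain is disconnected.
; Test input cycles Scarf spells; applying spell effects is a stub.
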(event Input|EnhancedActionEvents|EnhancedInputActionTestProgressTurn
  (params (ActionValue :type Boolean) (ElapsedSeconds :type Float%20%28double-precision%29) (TriggeredSeconds :type Float%20%28double-precision%29) (InputAction :type Input%20Action%20Object%20Reference :default "/Game/Blueprints/Player/TestProgressTurn.TestProgressTurn"))
  (CallFunction|IncrementScarfIndex))

(event EventBeginPlay
  (Input|AddMappingContext (PlayerController|LocalPlayerSubsystems|GetEnhancedInputLocalPlayerSubsystem (Game|GetPlayerController 0)) "/Game/Blueprints/Player/Macramage_MappingContext.Macramage_MappingContext" 0 "(bIgnoreAllPressedKeysUntilRelease=True,bForceImmediately=False,bNotifyUserSettings=False)")
  (Variables|Default|SetbShowMouseCursor true))

(event EventTick
  (params (DeltaSeconds :type Float%20%28single-precision%29))
  (switch Utilities|FlowControl|Switch|SwitchonTurnPhaseEnum (Variables|Default|GetTurnPhase)
    (:NewEnumerator3
      (CallFunction|GetTargetedIndexesScarfSpell true))))

(event Input|KeyboardEvents|X
  (params (Key :type Key%20Structure :default "None"))
  (:Pressed
    (bind _asmacramage_game_instance (Utilities|Casting|CastToMacramageGameInstance (Game|GetGameInstance)))
    (Development|PrintString (Utilities|String|ToString(Name) (Variables|/Game/Blueprints/Player/MacramageGameInstance.MacramageGameInstance_C|GetTest _asmacramage_game_instance)))))

(fn ConstructionScript)

(fn MovePhase
  (bind _gridreference (Variables|References|GetGridReference))
  (bind _gridreference_2 (Variables|References|GetGridReference))
  (bind _gridpoints (Variables|/Game/Blueprints/BP_Grid.BP_Grid_C|GetGridPoints _gridreference))
  (bind _gridpoints_2 (Variables|/Game/Blueprints/BP_Grid.BP_Grid_C|GetGridPoints _gridreference_2))
  (for _array_element (Variables|References|GetObjectArray)
    (bind _output_get (LocalVariables|SetEnemy%20Being%20Moved _array_element))
    (LocalVariables|SetGrid%20Point%20To%20MOve%20To (- (Variables|/Game/Blueprints/BP_ObjectParent.BP_ObjectParent_C|GetCurrentGridPoint _output_get) (* (Variables|/Game/Blueprints/BP_ObjectParent.BP_ObjectParent_C|GetMovementSpeed _output_get) (Variables|/Game/Blueprints/BP_Grid.BP_Grid_C|GetRows _gridreference_2))))
    ;[1 1 1] Check if in array
    (if (and (>= (- (Variables|/Game/Blueprints/BP_ObjectParent.BP_ObjectParent_C|GetCurrentGridPoint _output_get) (* (Variables|/Game/Blueprints/BP_ObjectParent.BP_ObjectParent_C|GetMovementSpeed _output_get) (Variables|/Game/Blueprints/BP_Grid.BP_Grid_C|GetRows _gridreference_2))) 0) (< (- (Variables|/Game/Blueprints/BP_ObjectParent.BP_ObjectParent_C|GetCurrentGridPoint _output_get) (* (Variables|/Game/Blueprints/BP_ObjectParent.BP_ObjectParent_C|GetMovementSpeed _output_get) (Variables|/Game/Blueprints/BP_Grid.BP_Grid_C|GetRows _gridreference_2))) (Utilities|Map|Length _gridpoints_2)))
      (bind _values (Utilities|Map|Values _gridpoints_2))
      ;[1 1 1] Check if space occupied
      (if (Utilities|Array|Get(acopy) _values (LocalVariables|GetGrid%20Point%20To%20MOve%20To))
        (Development|PrintString "Move Phase, Space to move to is Occupied")
        (else
          (Development|PrintString "Moving")
          (bind _keys (Utilities|Map|Keys _gridpoints))
          (Utilities|Map|Values _gridpoints)
          ;[1 1 1] Set old pos to empty
          (Utilities|Map|Add _gridpoints (Utilities|Array|Get(acopy) _keys (Variables|/Game/Blueprints/BP_ObjectParent.BP_ObjectParent_C|GetCurrentGridPoint (LocalVariables|GetEnemy%20Being%20Moved))) false)
          ;[1 1 1] Set New Pos to Occupied
          (Utilities|Map|Add _gridpoints (Utilities|Array|Get(acopy) _keys (LocalVariables|GetGrid%20Point%20To%20MOve%20To)) true)
          ;[1 1 1] Move to new pos
          (Default|Move (LocalVariables|GetEnemy%20Being%20Moved) (Transformation|GetWorldLocation (Utilities|Array|Get(acopy) _keys (LocalVariables|GetGrid%20Point%20To%20MOve%20To))) (LocalVariables|GetGrid%20Point%20To%20MOve%20To))))
      (else
        (Development|PrintString "Phase Move, Wants to leave grid space or atk"))))
  (return true))

(fn SpawnPhase
  (bind _outrownames (DataTable|GetDataTableRowNames "/Game/Blueprints/Data/Test_Level_Table.Test_Level_Table"))
  (bind _returnvalue (Utilities|GetDataTableRow "/Game/Blueprints/Data/Test_Level_Table.Test_Level_Table" (Utilities|Array|Get(acopy) _outrownames (Variables|Default|GetCurrentBackRow)))
    (:then
      (CallFunction|SpawnEnemy (.column1 _returnvalue) 1)
      (CallFunction|SpawnEnemy (.column2 _returnvalue) 2)
      (CallFunction|SpawnEnemy (.column3 _returnvalue) 3)
      (CallFunction|SpawnEnemy (.column4 _returnvalue) 4)
      (CallFunction|SpawnEnemy (.column5 _returnvalue) 5))
    (:RowNotFound
      (Development|PrintString "Error, Reached end of Rows in data table"))))

(fn SpawnEnemy
  (params (EnemyType :type MonsterEnum%20Enum :default "NewEnumerator0") (Collumn :type Integer))
  (bind _returnvalue (- Collumn 1))
  (bind _gridreference (Variables|References|GetGridReference))
  (bind _rows (Variables|/Game/Blueprints/BP_Grid.BP_Grid_C|GetRows _gridreference))
  (bind _collumns (Variables|/Game/Blueprints/BP_Grid.BP_Grid_C|GetCollumns _gridreference))
  (bind _gridpoints (Variables|/Game/Blueprints/BP_Grid.BP_Grid_C|GetGridPoints _gridreference))
  (bind _returnvalue_2 (- _rows 1))
  (bind _returnvalue_3 (* _returnvalue_2 _collumns))
  (bind _returnvalue_4 (+ _returnvalue _returnvalue_3))
  (bind _keys (Utilities|Map|Keys _gridpoints))
  (bind _values (Utilities|Map|Values _gridpoints))
  (Utilities|Array|SetArrayElem _values _returnvalue_4 true)
  (switch Utilities|FlowControl|Switch|SwitchonMonsterEnum EnemyType
    (:NewEnumerator1
      _)
    (:NewEnumerator2
      _))
  (bind _returnvalue_5 (Game|SpawnActorfromClass "/Game/Blueprints/BP_ObjectParent.BP_ObjectParent_C" (Math|Transform|MakeTransform (Transformation|GetWorldLocation (Utilities|Array|Get(acopy) _keys _returnvalue_4)) "0, 0, 0" "1.000000,1.000000,1.000000") "Undefined" "MultiplyWithRoot" 0 _returnvalue_4 EnemyType 0))
  (Utilities|Array|Add (Variables|References|GetObjectArray) _returnvalue_5))

(fn GetGridUnderCursor
  (bind (_success _index) (Class|GridPointInterface|GetIndex(Message) (.HitActor (Collision|BreakHitResult (.HitResult (Game|Player|GetHitResultUnderCursorbyChannel "TraceTypeQuery3" true))))))
  (return _success _index))

(fn GetShapeAroundPoint
  (params (Shape :type Array%20of%20Coordinate%20Struct%20Structures) (CenterIndex :type Integer) (CanWrap :type Boolean))
  (bind _gridreference (Variables|References|GetGridReference))
  (bind _gridreference_2 (Variables|References|GetGridReference))
  (bind _collumns (Variables|/Game/Blueprints/BP_Grid.BP_Grid_C|GetCollumns _gridreference))
  (bind _collumns_2 (Variables|/Game/Blueprints/BP_Grid.BP_Grid_C|GetCollumns _gridreference_2))
  (LocalVariables|SetCenter CenterIndex)
  (for _array_element Shape
    (bind _output_get (LocalVariables|SetTheoreticalIndex (+ (LocalVariables|GetCenter) (+ (* (.RowF-B (Utilities|Struct|BreakCoordinateStruct _array_element)) (Variables|/Game/Blueprints/BP_Grid.BP_Grid_C|GetCollumns (Variables|References|GetGridReference))) (.CollumnL-R (Utilities|Struct|BreakCoordinateStruct _array_element))))))
    (if (>= _output_get 0)
      (if (== (+ (/ (LocalVariables|GetCenter) _collumns_2) (.RowF-B (Utilities|Struct|BreakCoordinateStruct _array_element))) (/ (LocalVariables|GetTheoreticalIndex) _collumns_2))
        ;[1 1 1] Check if valid index
        (if (and (>= (LocalVariables|GetTheoreticalIndex) 0) (< (LocalVariables|GetTheoreticalIndex) (Utilities|Map|Length (Variables|/Game/Blueprints/BP_Grid.BP_Grid_C|GetGridPoints (Variables|References|GetGridReference))))) :!label _label
          (Utilities|Array|AddUnique (LocalVariables|GetEffectedIndexes) (LocalVariables|GetTheoreticalIndex)))
        (else
          ;[1 1 1] Invalidate or shift when goes over edge
          (if CanWrap
            ;;[1 1 1] Offset index by # of rows off, * amount per row
            (LocalVariables|SetTheoreticalIndex (- (LocalVariables|GetTheoreticalIndex) (* (Variables|/Game/Blueprints/BP_Grid.BP_Grid_C|GetCollumns _gridreference_2) (- (/ (LocalVariables|GetTheoreticalIndex) _collumns_2) (+ (/ (LocalVariables|GetCenter) _collumns_2) (.RowF-B (Utilities|Struct|BreakCoordinateStruct _array_element)))))))
            (goto _label))))
      (else
        ;[1 1 1] Wrapping in negatives, not gonna do full verticle wrap, just horizontal wrap and "rescue" values from -1 to -5
        (if CanWrap
          (if (not (== (+ (/ (LocalVariables|GetCenter) _collumns) (.RowF-B (Utilities|Struct|BreakCoordinateStruct _array_element))) (- (/ (LocalVariables|GetTheoreticalIndex) _collumns) 1)))
            (LocalVariables|SetTheoreticalIndex (+ (LocalVariables|GetTheoreticalIndex) 5))
            (goto _label))))))
  (return (LocalVariables|GetEffectedIndexes)))

(fn HighlightGridPoints
  (params (Points%20To%20Highlight :type Array%20of%20Integers))
  (for _array_element Points%20To%20Highlight
    (Default|HighlightPoint (Utilities|Array|Get(acopy) (Variables|/Game/Blueprints/BP_Grid.BP_Grid_C|GetGridPointIndecatiors (Variables|References|GetGridReference)) _array_element))))

(fn IncrementScarfIndex
  (bind _result (Math|Integer|IncrementInt (Variables|Default|GetScarfIndex))
    (:%20%20
      (if (== _result (Utilities|Array|Length (Variables|Default|GetScarf)))
        (Variables|Default|SetScarfIndex 0)))))

(fn GetTargetedIndexesScarfSpell
  (params (ShouldHighlight :type Boolean))
  (bind _scarf (Variables|Default|GetScarf))
  (bind _scarfindex (Variables|Default|GetScarfIndex))
  (bind _output (Utilities|Array|Get(acopy) _scarf _scarfindex))
  (bind (_effectedtilesshape _manacost _damage _additionaleffect _wrapping) (Utilities|Struct|BreakSpellStruct _output))
  (bind (_success _index) (CallFunction|GetGridUnderCursor))
  (if _success
    ;[1 1 1] Within castings distance
    (if (< _index (* (Variables|/Game/Blueprints/BP_Grid.BP_Grid_C|GetCollumns (Variables|References|GetGridReference)) (Variables|Default|GetCastingRange)))
      (if (Utilities|Array|IsNotEmpty _scarf)
        (bind _pointarray (CallFunction|GetShapeAroundPoint _effectedtilesshape _index _wrapping))
        (if ShouldHighlight
          (CallFunction|HighlightGridPoints _pointarray)
          (return _pointarray))))))

(fn EffectActorsonPointsScarfSpell
  (params (EffectedIndexes :type Array%20of%20Integers))
  ;[1 1 1] True if Object position is among effected tiles
  (for _array_element (Variables|References|GetObjectArray)
    (if (Utilities|Array|ContainsItem EffectedIndexes (Variables|/Game/Blueprints/BP_ObjectParent.BP_ObjectParent_C|GetCurrentGridPoint _array_element))
      _)))