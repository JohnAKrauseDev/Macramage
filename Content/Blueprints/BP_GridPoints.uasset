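; BP_GridPoints is an actor that lays out a columns-by-rows grid of points and registers itself with BP_Macramage_Controller on BeginPlay.
; RefreshGridIndecators spawns scene components spaced from GridStart and stores them as GridPoints map keys, each with a false flag.
; It optionally adds a static mesh indicator at each point.
; The refresh runs on BeginPlay, and in the construction script when UpdateInOutline is set.
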(event EventBeginPlay
  (CallFunction|RefreshGrid+Indecators)
  (bind _asbp_macramage_controller (Utilities|Casting|CastToBP_Macramage_Controller (Game|GetPlayerController 0)))
  (Variables|/Game/Blueprints/Player/BP_Macramage_Controller.BP_Macramage_Controller_C|SetGridReference _asbp_macramage_controller self))

(event Collision|EventActorBeginOverlap
  (params (OtherActor :type Actor%20Object%20Reference)))

(event EventTick
  (params (DeltaSeconds :type Float%20%28single-precision%29)))

(fn ConstructionScript
  (if (Variables|Default|GetUpdateInOutline)
    (CallFunction|RefreshGrid+Indecators)))

(fn RefreshGrid+Indecators
  ;[1 1 1] Clear old
  (bind _keys (Utilities|Map|Keys (Variables|Default|GetGridPoints)))
  (for _array_element _keys
    (Components|DestroyComponent _array_element))
  (for _array_element_2 (Variables|Default|GetGridPointIndecatiors)
    (Components|DestroyComponent _array_element_2))
  (bind _keys_2 (Utilities|Map|Keys (Variables|Default|GetGridPoints)))
  (Utilities|Array|Clear _keys_2)
  (Utilities|Array|Clear (Variables|Default|GetGridPointIndecatiors))
  (for _index (range 0 (- (Variables|Default|GetCollumns) 1))
    (for _index_2 (range 0 (- (Variables|Default|GetRows) 1))
      (bind _returnvalue (AddComponent|AddSceneComponent false (Math|Transform|MakeTransform (+ (Variables|/Script/Engine.SceneComponent|GetRelativeLocation (Variables|Default|GetGridStart)) (Math|Vector|MakeVector (* (Variables|Default|GetCollumnDistance) _index) (* _index_2 (Variables|Default|GetRowDistance)) 0.0)) "0, 0, 0" "1.000000,1.000000,1.000000")))
      (Utilities|Map|Add (Variables|Default|GetGridPoints) _returnvalue false)))
  (if (Variables|Default|GetShowIndecators)
    (bind _keys_3 (Utilities|Map|Keys (Variables|Default|GetGridPoints)))
    (for _array_element_3 _keys_3
      (AddComponent|AddStaticMeshComponent false (Transformation|GetRelativeTransform _array_element_3)))))